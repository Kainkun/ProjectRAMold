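; Piston actor that slides its MovingMesh along Z between its starting height and MaxDistance above it.
; Extend and Retract set the Extending flag and derive MoveDirection from Speed, and BeginPlay applies whichever state Extending starts in.
; Tick offsets the mesh locally without sweep, scaled by delta time, until it passes the limit for the current state, with no clamping or automatic reversal.
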(event `self.ReceiveBeginPlay`
  (set `self.StartPosition` (.z (`SceneComponent.RelativeLocation` (`self.MovingMesh`))))
  (if (`self.Extending`)
    (`self.Extend`)
    (else
      (`self.Retract`))))

(event `self.ReceiveTick`
  (params (DeltaSeconds :type "Float (single-precision)"))
  (set `self.MoveDelta` (- (.z (`SceneComponent.RelativeLocation` (`self.MovingMesh`))) (`self.StartPosition`)))
  (if (`self.Extending`)
    (if (< (`self.MoveDelta`) (`self.MaxDistance`))
      (`SceneComponent.K2_AddLocalOffset` (`self.MovingMesh`) (`KismetMathLibrary.MakeVector` 0.0 0.0 (* DeltaSeconds (`self.MoveDirection`))) false false :!label _label))
    (elif (> (`self.MoveDelta`) 0.0)
      (goto _label))))

(fn `Extend`
  (set `self.Extending` true)
  (set `self.MoveDirection` (`self.Speed`)))

(fn `Retract`
  (set `self.Extending` false)
  (bind _result (`/Engine/EditorBlueprintResources/StandardMacros.NegateFloat` (`self.Speed`))
    (:`  `
      (set `self.MoveDirection` _result))))

(fn `UserConstructionScript`)